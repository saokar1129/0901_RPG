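; BP_person is the player character, with camera-relative planar movement, sprint, weapon draw/sheathe and a melee combo.
; The weapon input toggles 拿武器, plays a montage, then after a delay reattaches component F to H or K and calls MoveComponentTo.
; Attacks require the weapon out and alternate two montages by counter parity, gated by a DoOnce with timed reset.
; BeginPlay adds the BW_介面 UI; 切換移動 sets the flag that gates movement.
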(event EventBeginPlay
  ;[1 1 1] 添加介面
  (bind _returnvalue (UserInterface|CreateWidget "/Game/BP/BW_介面.BW_介面_C" (Game|GetPlayerController 0)))
  (UserInterface|Viewport|AddtoViewport _returnvalue 0))

(event Input|ActionEvents|InputAction衝刺
  (params (Key :type Key%20Structure :default "None"))
  (bind _charactermovement (Variables|Character|GetCharacterMovement))
  ;[1 1 1] Comment
  (:Pressed
    (Variables|/Script/Engine.CharacterMovementComponent|SetMaxWalkSpeed _charactermovement 1e+03))
  (:Released
    (Variables|/Script/Engine.CharacterMovementComponent|SetMaxWalkSpeed _charactermovement 6e+02)))

(event Input|ActionEvents|InputAction武器
  (params (Key :type Key%20Structure :default "None"))
  (bind _f (Variables|Default|GetF))
  ;[1 1 1] Comment
  (:Pressed
    (Variables|Default|Set拿武器 (not (Variables|Default|Get拿武器)))
    (Animation|Montage|PlayMontage (Variables|Character|GetMesh) "/Game/animation/weapon_Montage.weapon_Montage"
      (:then
        (if (Variables|Default|Get拿武器)
          (Utilities|FlowControl|Delay 0.6)
          (Transformation|AttachComponentToComponent _f (Variables|Default|GetH) "None" "KeepRelative" "KeepRelative" "KeepRelative" true)
          (else
            (Utilities|FlowControl|Delay 0.5)
            (Transformation|AttachComponentToComponent _f (Variables|Default|GetK) "None" "KeepRelative" "KeepRelative" "KeepRelative" true)))
        (Components|MoveComponentTo _f "0, 0, 0" "0, 0, 0" false false 0.2 false)))))

(event Input|ActionEvents|InputAction攻擊1
  (params (Key :type Key%20Structure :default "None"))
  ;[1 1 1] Comment
  (:Pressed
    (Utilities|FlowControl|DoOnce false :!label _label
      (:Completed
        (if (Variables|Default|Get拿武器)
          (Animation|Montage|PlayMontage (Variables|Character|GetMesh) (Utilities|Select :Index (Math|Integer|%(Integer) (Variables|Default|Get攻擊1次數) 2) :Option%200 "/Game/animation/攻擊1_Montage.攻擊1_Montage" :Option%201 "/Game/animation/攻擊2_Montage.攻擊2_Montage") 2.0
            (:then
              (Math|Integer|IncrementInt (Variables|Default|Get攻擊1次數)
                (:%20%20
                  (Utilities|FlowControl|Delay 0.6)
                  (Utilities|FlowControl|Sequence
                    (:then_0
                      (goto _label Reset))
                    (:then_1
                      (Utilities|FlowControl|Delay 0.7)
                      (Variables|Default|Set攻擊1次數 0)))))))
          (else
            (goto _label Reset)))))))

(event Input|AxisEvents|InputAxisLookUp
  (params (AxisValue :type Float%20%28single-precision%29))
  ;[1 1 1] 滑鼠輸入
  (Pawn|Input|AddControllerPitchInput AxisValue))

(event Input|AxisEvents|InputAxisTurn
  (params (AxisValue :type Float%20%28single-precision%29))
  ;[1 1 1] 滑鼠輸入
  (Pawn|Input|AddControllerYawInput AxisValue))

(event Input|AxisEvents|InputAxisMoveForward
  (params (AxisValue :type Float%20%28single-precision%29))
  ;[1 1 1] 移動
  (if (Variables|Default|Get移動)
    (Pawn|Input|AddMovementInput (Math|Vector|GetForwardVector (Math|Rotator|MakeRotator 0.0 0.0 (.Yaw (Math|Rotator|BreakRotator (Pawn|GetControlRotation :!class /Script/Engine.Pawn))))) AxisValue false)))

(event Input|AxisEvents|InputAxisMoveRight
  (params (AxisValue :type Float%20%28single-precision%29))
  ;[1 1 1] 移動
  (if (Variables|Default|Get移動)
    (Pawn|Input|AddMovementInput (Math|Vector|GetRightVector (Math|Rotator|MakeRotator 0.0 0.0 (.Yaw (Math|Rotator|BreakRotator (Pawn|GetControlRotation :!class /Script/Engine.Pawn))))) AxisValue false)))

(fn ConstructionScript)

(fn 切換移動
  (params (移動 :type Boolean))
  (Variables|Default|Set移動 移動))